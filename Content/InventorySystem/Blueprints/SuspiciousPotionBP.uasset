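; Suspicious potion pickup that spins in the world, adds itself to the FPS_Controller's inventory on Interact, plays an equip sound and destroys itself.
; On use, a random stream, seeded at BeginPlay, picks either a capped heal or a penalty.
; The heal updates Health and the widget, while the penalty only sends a reduced value to the widget without changing Health.
; Each outcome sets its own GenericGameInstance flag.
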(event `/Game/InventorySystem/Interact.Interact`
  ;[0.06274 0.698 1 1 60] Aiste
  ;;[1 1 1] Adds Item to Inventory and plays a sound
  (bind _asfps_controller (cast `/Game/Assets/MainCharacter/FPS_Controller` (`GameplayStatics.GetPlayerCharacter` 0)))
  (`/Game/InventorySystem/Widgets/Inventory.AddToInventory` (`/Game/Assets/MainCharacter/FPS_Controller.InventoryWG` _asfps_controller) (`self.Item_Info`))
  (`GameplayStatics.PlaySoundAtLocation` "/Game/Audio/Sounds/Equip.Equip" (`SceneComponent.K2_GetComponentLocation` (`self.Sphere`)) (struct) 1.0 1.0 0.0 null null null null)
  (`self.K2_DestroyActor`))

(event `/Game/InventorySystem/Interact.UseItem`
  (bind _returnvalue (`GameplayStatics.GetPlayerCharacter` 0))
  ;[0.06274 0.698 1 1 60] Aiste
  ;;[1 1 1] Updates the health bar after consuming the suspicious potion
  (if (`KismetMathLibrary.RandomBoolFromStream` (`self.Random Stream Variable`))
    (bind _asfps_controller (cast `/Game/Assets/MainCharacter/FPS_Controller` _returnvalue))
    (bind _returnvalue_2 (+ (`/Game/Assets/MainCharacter/FPS_Controller.Health` _asfps_controller) 30.0))
    (if (<= _returnvalue_2 100.0)
      (set `/Game/Assets/MainCharacter/FPS_Controller.Health` _returnvalue_2 _asfps_controller)
      (else
        (set `/Game/Assets/MainCharacter/FPS_Controller.Health` 100.0 _asfps_controller)))
    (bind _asfps_controller_2 (cast `/Game/Assets/MainCharacter/FPS_Controller` (`GameplayStatics.GetPlayerCharacter` 0)))
    (`/Game/Assets/MainCharacter/User_Interface/HUD.Health Update` (`/Game/Assets/MainCharacter/FPS_Controller.PlayerWidgetRef` _asfps_controller_2) (`/Game/Assets/MainCharacter/FPS_Controller.Health` _asfps_controller_2))
    (bind _asgeneric_game_instance (cast `/Game/UI/GenericGameInstance` (`GameplayStatics.GetGameInstance`)))
    (set `/Game/UI/GenericGameInstance.HasAddedHealth?` true _asgeneric_game_instance)
    (else
      (bind _asfps_controller_3 (cast `/Game/Assets/MainCharacter/FPS_Controller` _returnvalue))
      (`/Game/Assets/MainCharacter/User_Interface/HUD.Health Update` (`/Game/Assets/MainCharacter/FPS_Controller.PlayerWidgetRef` _asfps_controller_3) (- (`/Game/Assets/MainCharacter/FPS_Controller.Health` _asfps_controller_3) 10.0))
      (bind _asgeneric_game_instance_2 (cast `/Game/UI/GenericGameInstance` (`GameplayStatics.GetGameInstance`)))
      (set `/Game/UI/GenericGameInstance.HasTakenHealth?` true _asgeneric_game_instance_2))))

(event `self.ReceiveTick`
  (params (DeltaSeconds :type "Float (single-precision)"))
  ;[0.06274 0.698 1 1 60] Aiste
  ;;[1 1 1] Rotation (cosmetic)
  (`SceneComponent.K2_AddLocalRotation` (`self.DefaultSceneRoot`) (`KismetMathLibrary.MakeRotator` 0.0 0.0 (+ DeltaSeconds 3.0)) false false))

(event `self.ReceiveBeginPlay`
  ;[0.06274 0.698 1 1 60] Aiste
  ;;[1 1 1] Set random chance seed
  (`KismetMathLibrary.SeedRandomStream` (`self.Random Stream Variable`))
  (set `self.Chance` (`KismetMathLibrary.RandomBoolFromStream` (`self.Random Stream Variable`))))

(fn `UserConstructionScript`
  (`parent.UserConstructionScript`))