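; Health potion pickup for the inventory system that restores player health when used.
; Interact adds its item info to the FPS_Controller inventory widget, plays an equip sound and destroys the actor.
; UseItem raises the player's HealthMax, which serves as current health, by a fixed amount up to a cap, then updates the health bar.
; Tick applies a cosmetic yaw spin that adds DeltaSeconds rather than scaling by it, so speed depends on frame rate.
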(event `/Game/InventorySystem/Interact.Interact`
  ;[0.06274 0.698 1 1 60] Aiste
  ;;[1 1 1] Adds Item to Inventory and plays a sound
  (bind _asfps_controller (cast `/Game/Assets/MainCharacter/FPS_Controller` (`GameplayStatics.GetPlayerCharacter` 0)))
  (`/Game/InventorySystem/Widgets/Inventory.AddToInventory` (`/Game/Assets/MainCharacter/FPS_Controller.InventoryWG` _asfps_controller) (`self.Item_Info`))
  (`GameplayStatics.PlaySoundAtLocation` "/Game/Audio/Sounds/Equip.Equip" (`SceneComponent.K2_GetComponentLocation` (`self.Sphere`)) (struct) 1.0 1.0 0.0 null null null null)
  (`self.K2_DestroyActor`))

(event `/Game/InventorySystem/Interact.UseItem`
  ;[0.06274 0.698 1 1 60] Aiste
  ;;[1 1 1] Updates the health bar after consuming the health pot
  (bind _asfps_controller (cast `/Game/Assets/MainCharacter/FPS_Controller` (`GameplayStatics.GetPlayerCharacter` 0)))
  (bind _returnvalue (+ (`/Game/Assets/MainCharacter/FPS_Controller.Health_Max` _asfps_controller) 10.0))
  (if (<= _returnvalue 100.0)
    (set `/Game/Assets/MainCharacter/FPS_Controller.Health_Max` _returnvalue _asfps_controller)
    (else
      (set `/Game/Assets/MainCharacter/FPS_Controller.Health_Max` 100.0 _asfps_controller)))
  (bind _asfps_controller_2 (cast `/Game/Assets/MainCharacter/FPS_Controller` (`GameplayStatics.GetPlayerCharacter` 0)))
  (`/Game/Assets/MainCharacter/User_Interface/HUD.Health Update` (`/Game/Assets/MainCharacter/FPS_Controller.PlayerWidgetRef` _asfps_controller_2) (`/Game/Assets/MainCharacter/FPS_Controller.Health_Max` _asfps_controller_2)))

(event `self.ReceiveTick`
  (params (DeltaSeconds :type "Float (single-precision)"))
  ;[0.06274 0.698 1 1 60] Aiste
  ;;[1 1 1] Rotation (cosmetic)
  (`SceneComponent.K2_AddLocalRotation` (`self.DefaultSceneRoot`) (`KismetMathLibrary.MakeRotator` 0.0 0.0 (+ DeltaSeconds 3.0)) false false))

(fn `UserConstructionScript`
  (`parent.UserConstructionScript`))