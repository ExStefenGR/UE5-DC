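; DoorKeyBP is a door key pickup that the player collects through an Interact event.
; Interacting adds its item info to the FPS_Controller character's inventory widget and plays an equip sound at the sphere component's location.
; It then sets HasKey on itself and on GenericGameInstance, keeping the flag available after the key actor destroys itself.
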(event `/Game/InventorySystem/Interact.Interact`
  ;[0.06274 0.698 1 1 90] Aiste
  ;;[1 1 1] Interaction with the key
  (bind _asfps_controller (cast `/Game/Assets/MainCharacter/FPS_Controller` (`GameplayStatics.GetPlayerCharacter` 0)))
  (`/Game/InventorySystem/Widgets/Inventory.AddToInventory` (`/Game/Assets/MainCharacter/FPS_Controller.InventoryWG` _asfps_controller) (`self.Item_Info`))
  (set `self.HasKey?` true)
  (`GameplayStatics.PlaySoundAtLocation` "/Game/Audio/Sounds/Equip.Equip" (`SceneComponent.K2_GetComponentLocation` (`self.Sphere`)) (struct) 1.0 1.0 0.0 null null null null)
  (bind _asgeneric_game_instance (cast `/Game/UI/GenericGameInstance` (`GameplayStatics.GetGameInstance`)))
  (set `/Game/UI/GenericGameInstance.HasKey?` (`self.HasKey?`) _asgeneric_game_instance)
  (`self.K2_DestroyActor`))

(fn `UserConstructionScript`
  (`parent.UserConstructionScript`))